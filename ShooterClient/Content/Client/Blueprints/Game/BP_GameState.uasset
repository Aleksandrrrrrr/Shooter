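; Game state that runs the match period, countdown timer and per-player kill/death scoreboard.
; Server events set the period and start a self-rearming one-second countdown; OnRep functions and an end-of-timer multicast fire dispatchers.
; Entering the Game period adds every player controller to GameData.
; On a death, SetArray updates victim and killer counts, then a multicast has remote machines broadcast each player's score through the CharacterDead dispatcher.
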(event Custom|StartTimer_Server
  (params (Timer :type Float%20%28double-precision%29))
  ;[0.8704 1 0] Timer
  (Variables|Default|SetTimer Timer)
  (Utilities|Time|SetTimerbyFunctionName 0 "CauntingTimer" 1.0))

(event Custom|TimerEnded_Server
  ;[0.8704 1 0] Timer
  (CallFunction|TimerEndedMulticast))

(event Custom|TimerEnded_Multicast
  ;[0.8704 1 0] Timer
  (Default|CallOnTimerEnded))

(event Custom|CharacterDead_Server
  (params (Player :type BP%20Player%20Controller%20Object%20Reference) (Character :type BP%20Player%20Character%20Object%20Reference) (Causer :type BP%20Player%20Character%20Object%20Reference))
  ;[0 0 0] Dead
  (CallFunction|SetArray Player Causer)
  (CallFunction|ChangeDataMulticast))

(event Custom|ChangeGamePeriod_Server
  (params (GamePeriod :type e_GamePeriod%20Enum :default "NewEnumerator0"))
  ;[0.2338 0.4113 1] Change game period
  (bind _output_get (Variables|Default|SetGamePeriod GamePeriod))
  (switch Utilities|FlowControl|Switch|Switchone_GamePeriod _output_get
    (:NewEnumerator1
      ;;[1 0 0] ToDo: Needs refactoring
      (bind _outactors (Actor|GetAllActorsOfClass "/Game/Client/Blueprints/Game/BP_PlayerController.BP_PlayerController_C"))
      (for _array_element _outactors
        (Utilities|Array|Add (Variables|Default|GetGameData) (Utilities|Struct|Makestr_PlayerData _array_element (Utilities|Text|ToText(Object) _array_element)))))))

(event Custom|ChangeData_Multicast
  ;[0 0 0] Dead
  (Networking|SwitchHasAuthority
    (:Remote
      (CallFunction|ChangedData))))

(event EventTick
  (params (DeltaSeconds :type Float%20%28single-precision%29))
  ;[1 0 0] DEBUG
)

(fn ConstructionScript)

(fn CauntingTimer
  (bind _result (Math|Float|DecrementFloat (Variables|Default|GetTimer))
    (:%20%20
      (if (<= _result 0.0)
        (CallFunction|TimerEndedServer)
        (else
          (Utilities|Time|SetTimerbyFunctionName 0 "CauntingTimer" 1.0))))))

(fn OnRepTimer
  (Default|CallOnTimerChanged (Variables|Default|GetGamePeriod) (Variables|Default|GetTimer)))

(fn OnRepGamePeriod
  (Default|CallOnChangeGamePeriod (Variables|Default|GetGamePeriod)))

(fn GetDatabyCharacterName
  (params (Name :type Text%20%28by%20ref%29))
  (for _array_element (Variables|Default|GetGameData)
    (if (Utilities|Enum|Equal(Enum) (Utilities|Struct|Breakstr_PlayerData _array_element) Name)
      (return _array_element)))
  (return ""))

(fn ChangedData
  (for _array_element (Variables|Default|GetGameData)
    (Default|CallOnCharacterDead (.playername _array_element) (.kill _array_element) (.dead _array_element))))

(fn SetArray
  (params (Player :type Object%20Object%20Reference) (Causer :type Pawn%20Object%20Reference))
  (for (_array_element _array_index) (Variables|Default|GetGameData)
    (LocalVariables|SetLocalData _array_element)
    (LocalVariables|SetIndex _array_index)
    (if (== Player (Utilities|Struct|Breakstr_PlayerData _array_element))
      (Utilities|Array|SetArrayElem (Variables|Default|GetGameData) (LocalVariables|GetIndex) (Utilities|Struct|Makestr_PlayerData (.player (LocalVariables|GetLocalData)) (.playername (LocalVariables|GetLocalData)) (.kill (LocalVariables|GetLocalData)) (+ (.dead (LocalVariables|GetLocalData)) 1)))
      (else
        (bind _asbp_player_controller (Utilities|Casting|CastToBP_PlayerController (Pawn|GetController Causer)))
        (if (== _asbp_player_controller (.player (LocalVariables|GetLocalData)))
          (Utilities|Array|SetArrayElem (Variables|Default|GetGameData) (LocalVariables|GetIndex) (Utilities|Struct|Makestr_PlayerData _asbp_player_controller (.playername (LocalVariables|GetLocalData)) (+ (.kill (LocalVariables|GetLocalData)) 1) (.dead (LocalVariables|GetLocalData)))))))))