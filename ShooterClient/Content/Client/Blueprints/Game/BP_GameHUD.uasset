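; Game HUD that manages the player's start screen, in-game HUD, death screen and player table.
; Init creates the widgets and binds events from the pawn's weapons and health and from BP_GameState, which forward values to them.
; The Game period swaps start screen for HUD and fills the table.
; Death briefly shows a screen and rebuilds the HUD; stat updates rebind events after a delay marked ToDo.
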(event Custom|CharacterDead
  ;[1 0 0.3688] Character dead
  (Utilities|FlowControl|Sequence
    (:then_0
      ;;[0 0 0] Dead widget
      (bind _returnvalue (UserInterface|CreateWidget "/Game/Client/UI/WBP_DeadScreen.WBP_DeadScreen_C" (Game|Player|GetOwningPlayerController)))
      (bind _output_get (Variables|Default|SetDeadWidget _returnvalue))
      (UserInterface|Viewport|AddtoViewport _output_get 0)
      (Input|SetInputModeUIOnly (Game|Player|GetOwningPlayerController) _output_get "DoNotLock" false)
      (Widget|RemovefromParent (Variables|Default|GetHUD))
      (Utilities|FlowControl|Delay 2.0)
      (Widget|RemovefromParent (Variables|Default|GetDeadWidget)))
    (:then_1
      ;;[0 1 0.3734] Create new HUD
      (bind _hud (Variables|Default|GetHUD)
        (:then
          (Widget|RemovefromParent _hud))
        (:else
          _))
      (bind _returnvalue_2 (UserInterface|CreateWidget "/Game/Client/UI/WBP_HUD.WBP_HUD_C" (Game|Player|GetOwningPlayerController)))
      (bind _output_get_2 (Variables|Default|SetHUD _returnvalue_2))
      (UserInterface|Viewport|AddtoViewport _output_get_2 0)
      (Default|ChangeWeapon (Variables|Default|GetHUD) "NewEnumerator0")
      (Input|SetInputModeGameOnly (Game|Player|GetOwningPlayerController) false))))

(event Custom|ChangedGamePeriod
  (params (GamePeriod :type e_GamePeriod%20Enum :default "NewEnumerator0"))
  ;[1 0.9097 0] Game mode
  (bind _output_get (Variables|Default|SetGamePeriod GamePeriod))
  (switch Utilities|FlowControl|Switch|Switchone_GamePeriod _output_get
    (:NewEnumerator1
      (Widget|RemovefromParent (Variables|Default|GetStartScreen))
      (UserInterface|Viewport|AddtoViewport (Variables|Default|GetHUD) 0)
      (bind _asbp_game_state (Utilities|Casting|CastToBP_GameState (Game|GetGameState)))
      (CallFunction|CreateDataWidgetServer (Variables|/Game/Client/Blueprints/Game/BP_GameState.BP_GameState_C|GetGameData _asbp_game_state)))))

(event Custom|ChangeHealth
  (params (Current :type Float%20%28double-precision%29) (Max :type Float%20%28double-precision%29))
  ;[1 0.2753 0.09495] Change health
  (Default|ChangeHealth (Variables|Default|GetHUD) Current Max))

(event Custom|TimerChanged
  (params (GamePeriod :type e_GamePeriod%20Enum :default "NewEnumerator0") (CurrentTimer :type Float%20%28double-precision%29))
  ;[1 0.9097 0] Game mode
  (switch Utilities|FlowControl|Switch|Switchone_GamePeriod GamePeriod
    (:NewEnumerator0
      (Default|ChangeTimer (Variables|Default|GetStartScreen) CurrentTimer))
    (:NewEnumerator1
      (Default|ChangeTimer (Variables|Default|GetHUD) CurrentTimer))))

(event Custom|CreateDataWidget_Server
  (params (Data :type Array%20of%20Str%20Player%20Data%20Structures))
  ;[0.5272 0.114 1] Table of players
  (for _array_element Data
    (Default|AddPlayer (Variables|Default|GetTableOfPlayers) (Utilities|Struct|Breakstr_PlayerData _array_element))))

(event Custom|ChangeActiveWeapon
  (params (WeaponType :type e_WeaponType%20Enum :default "NewEnumerator0"))
  ;[0.1624 1 0.7049] Change weapon events
  (Default|ChangeWeapon (Variables|Default|GetHUD) WeaponType))

(event Custom|ChangeAmmo
  (params (CurrentAmmo :type Integer) (TotalAmmo :type Integer))
  ;[0.1624 1 0.7049] Change weapon events
  (Default|ChangeAmmo (Variables|Default|GetHUD) CurrentAmmo TotalAmmo))

(event Custom|ShowTableOfPlayers_Client
  (params (Show :type Boolean))
  ;[0.5272 0.114 1] Table of players
  (Widget|SetVisibility (Variables|Default|GetTableOfPlayers) (select Show "Visible" "Hidden")))

(event Custom|PlayerDataUpdate
  (params (CharacterName :type Text) (Kill :type Integer) (Dead :type Integer))
  ;[0.5272 0.114 1] Table of players
  (Default|UpdateStatistics (Variables|Default|GetTableOfPlayers) CharacterName (Utilities|Text|ToText(Integer) Kill) (Utilities|Text|ToText(Integer) Dead))
  ;;[1 0 0] ToDo
  (Utilities|FlowControl|Delay 3.0)
  (Internal|BindEventsNewCharacter))

(event EventBeginPlay
  ;[0.08416 1 0.483] Initial
  (Internal|Init))

(fn ConstructionScript)

(fn Init
  (CallFunction|CreateWidgets)
  (Internal|BindEventsNewCharacter))

(fn CreateWidgets
  (Utilities|FlowControl|Sequence
    (:then_0
      (bind _returnvalue (UserInterface|CreateWidget "/Game/Client/UI/WBP_HUD.WBP_HUD_C" (Game|Player|GetOwningPlayerController)))
      (Variables|Default|SetHUD _returnvalue)
      (Default|ChangeWeapon (Variables|Default|GetHUD) "NewEnumerator0"))
    (:then_1
      (bind _returnvalue_2 (UserInterface|CreateWidget "/Game/Client/UI/WBP_StartScreen.WBP_StartScreen_C" (Game|Player|GetOwningPlayerController)))
      (Variables|Default|SetStartScreen _returnvalue_2)
      (bind _returnvalue_3 (UserInterface|CreateWidget "/Game/Client/UI/WBP_TableOfPlayers.WBP_TableOfPlayers_C" (Game|Player|GetOwningPlayerController)))
      (Variables|Default|SetTableOfPlayers _returnvalue_3))
    (:then_2
      (UserInterface|Viewport|AddtoViewport (Variables|Default|GetStartScreen) 0)
      (UserInterface|Viewport|AddtoViewport (Variables|Default|GetTableOfPlayers) 1)
      (Widget|SetVisibility (Variables|Default|GetTableOfPlayers) "Hidden"))))

(fn BindEventsNewCharacter
  (Utilities|FlowControl|Sequence
    (:then_0
      ;[0.2104 0.2231 1] Bind weapons
      (bind _asbp_player_character (Utilities|Casting|CastToBP_PlayerCharacter (Class|HUD|GetOwningPawn)))
      (EventDispatchers|BindEventtoOnChangeActiveWeapon (Variables|/Game/Client/Blueprints/Game/BP_PlayerCharacter.BP_PlayerCharacter_C|GetWeaponsManager _asbp_player_character) (EventDispatchers|CreateEvent :!event Custom|ChangeActiveWeapon))
      (EventDispatchers|BindEventtoOnChangeAmmo (Variables|/Game/Client/Blueprints/Game/BP_PlayerCharacter.BP_PlayerCharacter_C|GetWeaponsManager _asbp_player_character) (EventDispatchers|CreateEvent :!event Custom|ChangeAmmo)))
    (:then_1
      ;[1 0.07456 0.2549] Bind statistics
      (bind _asbp_player_character_2 (Utilities|Casting|CastToBP_PlayerCharacter (Class|HUD|GetOwningPawn)))
      (EventDispatchers|BindEventtoOnStatValueChanged (Variables|/Game/Client/Blueprints/Game/BP_PlayerCharacter.BP_PlayerCharacter_C|GetHealth _asbp_player_character_2) (EventDispatchers|CreateEvent :!event Custom|ChangeHealth)))
    (:then_2
      ;[1 0.7287 0.02728] Bind game mode
      (bind _asbp_game_state (Utilities|Casting|CastToBP_GameState (Game|GetGameState)))
      (EventDispatchers|BindEventtoOnTimerChanged _asbp_game_state (EventDispatchers|CreateEvent :!event Custom|TimerChanged))
      (EventDispatchers|BindEventtoOnChangeGamePeriod _asbp_game_state (EventDispatchers|CreateEvent :!event Custom|ChangedGamePeriod))
      (EventDispatchers|BindEventtoOnCharacterDead _asbp_game_state (EventDispatchers|CreateEvent :!event Custom|PlayerDataUpdate)))))