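; Game mode that runs the match flow from start countdown to timed session and handles player death and respawn.
; BP_GameState runs the server timers, and its timer-ended event drives the switch from Start to Game period.
; On death, the controller possesses a spawned BP_Spectator, the character is destroyed and the game state is notified.
; After a short delay, a new BP_PlayerCharacter spawns at a random PlayerStart.
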(event Custom|CharacterDead
  (params (PlayerController :type BP%20Player%20Controller%20Object%20Reference) (Character :type BP%20Player%20Character%20Object%20Reference) (Causer :type BP%20Player%20Character%20Object%20Reference))
  ;[1 0 0.4968] Character dead
  (Utilities|FlowControl|Sequence
    (:then_0
      (bind _returnvalue (Game|SpawnActorfromClass "/Game/Client/Blueprints/Game/BP_Spectator.BP_Spectator_C" (Math|Transform|MakeTransform "0, 0, 0" "0, 0, 0" "1.000000,1.000000,1.000000") "AlwaysSpawn" "MultiplyWithRoot" PlayerController Causer 0))
      (Pawn|Possess PlayerController _returnvalue)
      (Actor|DestroyActor Character))
    (:then_1
      (Utilities|FlowControl|Delay 2.0)
      (Internal|RespawnPlayer PlayerController))
    (:then_2
      (Default|CharacterDeadServer (Variables|Default|GetBPGameState) PlayerController Character Causer))))

(event Custom|TimerEnded
  ;[0.3974 0.156 1] Game session
  (switch Utilities|FlowControl|Switch|Switchone_GamePeriod (Variables|Default|GetGamePeriod)
    (:NewEnumerator0
      (CallFunction|StartSession))))

(event Custom|StartSession
  ;[0.3974 0.156 1] Game session
  (Default|StartTimerServer (Variables|Default|GetBPGameState) (Variables|Default|GetSessionTimer))
  (Default|ChangeGamePeriodServer (Variables|Default|GetBPGameState) "NewEnumerator1")
  (Variables|Default|SetGamePeriod "NewEnumerator1"))

(event EventBeginPlay
  ;[0 1 0.7554] Init
  (|CallParentFunction)
  (bind _asbp_game_state (Utilities|Casting|CastToBP_GameState (Game|GetGameState)))
  (bind _output_get (Variables|Default|SetBPGameState _asbp_game_state))
  (Default|StartTimerServer _output_get (Variables|Default|GetStartTimer))
  (EventDispatchers|BindEventtoOnTimerEnded (Variables|Default|GetBPGameState) (EventDispatchers|CreateEvent :!event Custom|TimerEnded)))

(fn ConstructionScript)

(fn TimerCaunting
  (bind _result (Math|Float|DecrementFloat (Variables|Default|GetTimer))
    (:%20%20
      (Default|CallOnTimerChanged (Variables|Default|GetGamePeriod) _result)
      (if (<= (Variables|Default|GetTimer) 0.0)
        (CallFunction|TimerEnded)
        (else
          (Utilities|Time|SetTimerbyFunctionName 0 "TimerCaunting" 1.0))))))

(fn OnRepGamePeriod
  (Default|CallOnChangeGamePeriod (Variables|Default|GetGamePeriod)))

(fn RespawnPlayer
  (params (Player :type BP%20Player%20Controller%20Object%20Reference))
  (Utilities|FlowControl|Sequence
    (:then_0
      (Actor|DestroyActor (Pawn|GetControlledPawn Player)))
    (:then_1
      (bind _outactors (Actor|GetAllActorsOfClass "/Script/Engine.PlayerStart"))
      (bind _returnvalue (Game|SpawnActorfromClass "/Game/Client/Blueprints/Game/BP_PlayerCharacter.BP_PlayerCharacter_C" (Transformation|GetActorTransform (Utilities|Array|Get(acopy) _outactors (Math|Random|RandomInteger (Utilities|Array|LastIndex _outactors)))) "AlwaysSpawn" "MultiplyWithRoot" Player 0))
      (Pawn|Possess Player _returnvalue))))