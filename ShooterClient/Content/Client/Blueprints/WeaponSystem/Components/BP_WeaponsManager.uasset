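; Player character component that manages primary and secondary weapons, including spawning, switching, shooting and reloading.
; The server spawns BP_BaseWeapon actors from weapon definitions, then multicasts their attachment to first-person or third-person sockets based on local control.
; Server events switch the active weapon, whose RepNotify toggles visibility and notifies the client.
; Bindings to the active weapon's events feed the component's ammo and hit dispatchers.
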(event Custom|Hit
  (params (HitResult :type Hit%20Result%20Structure) (Damage :type Float%20%28double-precision%29))
  ;[1 0 0.04918] Hit result
  (Default|CallOnHit HitResult Damage))

(event Custom|AttachWeapon_Multicast
  (params (Weapon :type BP%20Base%20Weapon%20Object%20Reference%20%28by%20ref%29))
  (bind _playercharacter (Variables|Internal|GetPlayerCharacter))
  ;[0.2118 1 0.4018] Change weapon
  (Utilities|IsValid Weapon
    (:Is%20Valid
      (Transformation|AttachComponentToComponent Weapon (Default|GetVisibleMesh _playercharacter) (select (Pawn|IsLocallyControlled _playercharacter) "FP_Weapon" "TP_Weapon") "SnapToTarget" "SnapToTarget" "KeepRelative" true))))

(event Custom|ChangeWeapon_Server
  (params (Type :type e_WeaponType%20Enum :default "NewEnumerator0"))
  ;[0.2118 1 0.4018] Change weapon
  (if (CallFunction|PossibilityOfChangingWeapons Type)
    (CallFunction|UnbindChangeAmmoEvent)
    (CallFunction|SelectWeapon Type)
    (CallFunction|BindWeaponEvent)))

(event Custom|Reload_Server
  ;[0.1763 1 0.2049] Reload
  (Default|ReloadServer (Variables|Weapons|GetCurrentWeapon)))

(event Custom|CreateWeapon_Server
  (bind _value (Weapons|GetActiveWeapon))
  ;[0.2956 0.5492 1] Initial
  (for _array_element (Variables|Default|GetWeapons)
    (bind _weapon (CallFunction|CreateWeapon _array_element))
    (CallFunction|AttachWeaponMulticast _weapon))
  (CallFunction|SelectWeapon "NewEnumerator0")
  (CallFunction|BindWeaponEvent)
  ;[1 0 0] ToDo
  (Utilities|FlowControl|Delay 0.5)
  (CallFunction|ChangeAmmoClient (Variables|/Game/Client/Blueprints/WeaponSystem/Items/BP_BaseWeapon.BP_BaseWeapon_C|GetCurrentAmmo _value) (Variables|/Game/Client/Blueprints/WeaponSystem/Items/BP_BaseWeapon.BP_BaseWeapon_C|GetTotalAmmo _value)))

(event Custom|ChangeActiveWeapon_Client
  (params (WeaponType :type e_WeaponType%20Enum :default "NewEnumerator0"))
  ;[0.2118 1 0.4018] Change weapon
  (Default|CallOnChangeActiveWeapon WeaponType))

(event Custom|ChangeAmmo_Client
  (params (CurrentAmmo :type Integer) (TotalAmmo :type Integer))
  ;[1 0.4311 0] Ammo
  (Default|CallOnChangeAmmo CurrentAmmo TotalAmmo))

(event Custom|StopShooting_Server
  (bind _value (Weapons|GetActiveWeapon))
  ;[1 0.1521 0.7529] Shooting
  (Utilities|IsValid _value
    (:Is%20Valid
      (Default|StopShootingServer _value))))

(event Custom|Shot_Server
  (bind _value (Weapons|GetActiveWeapon))
  ;[1 0.1521 0.7529] Shooting
  (Utilities|IsValid _value
    (:Is%20Valid
      (Default|StartShotServer _value))))

(event EventBeginPlay
  ;[0.2956 0.5492 1] Initial
  (Internal|Init))

(event EventEndPlay
  (params (EndPlayReason :type EEndPlayReason%20Enum :default "Destroyed"))
  ;[0.2956 0.5492 1] Initial
  (|CallParentFunction EndPlayReason)
  (Utilities|FlowControl|Sequence
    (:then_0
      (bind _primaryweapon (Variables|Weapons|GetPrimaryWeapon)
        (:then
          (Actor|DestroyActor _primaryweapon))
        (:else)))
    (:then_1
      (bind _secondaryweapon (Variables|Weapons|GetSecondaryWeapon)
        (:then
          (Actor|DestroyActor _secondaryweapon))
        (:else)))))

(fn PossibilityOfChangingWeapons
  (params (WeaponIndex :type e_WeaponType%20Enum :default "NewEnumerator0"))
  (bind _primaryweapon (Variables|Weapons|GetPrimaryWeapon))
  (bind _secondaryweapon (Variables|Weapons|GetSecondaryWeapon))
  (bind _returnvalue (Utilities|Select :Index WeaponIndex :NewEnumerator0 _primaryweapon :NewEnumerator1 _secondaryweapon))
  (return (and (Utilities|IsValid _returnvalue) (!= _returnvalue (Variables|Weapons|GetCurrentWeapon)))))

(fn GetActiveWeapon
  (return (Variables|Weapons|GetCurrentWeapon)))

(fn CreateWeapon
  (params (WeaponDef :type Str%20Weapon%20Definition%20Structure))
  (bind _playercharacter (Variables|Internal|GetPlayerCharacter))
  (if (Networking|IsServer)
    (bind _returnvalue (Game|SpawnActorfromClass "/Game/Client/Blueprints/WeaponSystem/Items/BP_BaseWeapon.BP_BaseWeapon_C" (Math|Transform|MakeTransform "0, 0, 0" "0, 0, 0" "1.000000,1.000000,1.000000") "AlwaysSpawn" "MultiplyWithRoot" (Pawn|GetController _playercharacter) WeaponDef _playercharacter))
    (bind _output_get (LocalVariables|SetCreatedWeapon _returnvalue))
    (Transformation|AttachActorToActor _output_get (Variables|Internal|GetPlayerCharacter) "None" "SnapToTarget" "SnapToTarget" "KeepRelative" true)
    (Utilities|FlowControl|Sequence
      (:then_0
        (switch Utilities|FlowControl|Switch|Switchone_WeaponType (.Type (Utilities|Struct|Breakstr_WeaponDefinition WeaponDef))
          (:NewEnumerator0
            (CallFunction|SingletonWeapon (Variables|Weapons|GetPrimaryWeapon))
            (Variables|Weapons|SetPrimaryWeapon (LocalVariables|GetCreatedWeapon)))
          (:NewEnumerator1
            (CallFunction|SingletonWeapon (Variables|Weapons|GetSecondaryWeapon))
            (Variables|Weapons|SetSecondaryWeapon (LocalVariables|GetCreatedWeapon)))))
      (:then_1
        (return (LocalVariables|GetCreatedWeapon))))))

(fn Init
  (bind _asbp_player_character (Utilities|Casting|CastToBP_PlayerCharacter (Components|GetOwner)))
  (Variables|Internal|SetPlayerCharacter _asbp_player_character))

(fn SelectWeapon
  (params (Weapon :type e_WeaponType%20Enum :default "NewEnumerator0"))
  (switch Utilities|FlowControl|Switch|Switchone_WeaponType Weapon
    (:NewEnumerator0
      (Variables|Weapons|SetCurrentWeapon (Variables|Weapons|GetPrimaryWeapon)))
    (:NewEnumerator1
      (Variables|Weapons|SetCurrentWeapon (Variables|Weapons|GetSecondaryWeapon)))))

(fn OnRepCurrentWeapon
  (Utilities|FlowControl|Sequence
    (:then_0
      (bind _secondaryweapon (Variables|Weapons|GetSecondaryWeapon)
        (:then
          (Rendering|SetActorHiddenInGame _secondaryweapon (!= _secondaryweapon (Variables|Weapons|GetCurrentWeapon))))
        (:else)))
    (:then_1
      (bind _primaryweapon (Variables|Weapons|GetPrimaryWeapon)
        (:then
          (Rendering|SetActorHiddenInGame _primaryweapon (!= _primaryweapon (Variables|Weapons|GetCurrentWeapon))))
        (:else)))
    (:then_2
      (bind _currentweapon (Variables|Weapons|GetCurrentWeapon)
        (:then
          (CallFunction|ChangeActiveWeaponClient (Utilities|Struct|Breakstr_WeaponDefinition (Variables|/Game/Client/Blueprints/WeaponSystem/Items/BP_BaseWeapon.BP_BaseWeapon_C|GetWeaponDefinition _currentweapon))))
        (:else)))))

(fn BindWeaponEvent
  (bind _value (Weapons|GetActiveWeapon))
  (EventDispatchers|BindEventtoOnReload _value (EventDispatchers|CreateEvent :!event Custom|ChangeAmmo_Client))
  (EventDispatchers|BindEventtoOnChangeAmmo _value (EventDispatchers|CreateEvent :!event Custom|ChangeAmmo_Client))
  (EventDispatchers|BindEventtoOnHit _value (EventDispatchers|CreateEvent :!event Custom|Hit)))

(fn UnbindChangeAmmoEvent
  (bind _value (Weapons|GetActiveWeapon))
  (EventDispatchers|UnbindEventfromOnReload _value (EventDispatchers|CreateEvent :!event Custom|ChangeAmmo_Client))
  (EventDispatchers|UnbindEventfromOnChangeAmmo _value (EventDispatchers|CreateEvent :!event Custom|ChangeAmmo_Client)))

(fn SingletonWeapon
  (params (InputPin :type BP%20Base%20Weapon%20Object%20Reference))
  (Utilities|IsValid InputPin
    (:Is%20Valid
      (Actor|DestroyActor InputPin)
      (return))
    (:Is%20Not%20Valid
      (return))))