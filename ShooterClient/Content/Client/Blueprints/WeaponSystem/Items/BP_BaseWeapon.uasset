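; Networked base weapon for player characters, configured by a WeaponDefinition for ammo, timing, damage and animations.
; Server events gate fire and reload with cooldown flags and timers, looping shots for automatic weapons and auto-reloading when empty.
; Shots line-trace from the camera and report hits and ammo changes through dispatchers.
; Multicasts play animations on remote-role instances, choosing montages by local control, and draw a debug sphere at each hit.
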(event Custom|Shot_Multicast
  (bind _weapondefinition (Variables|Default|GetWeaponDefinition))
  (bind (_shotanimation_weapon _shotanimation_character) (Utilities|Struct|Breakstr_WeaponDefinition _weapondefinition))
  ;[0.9702 0.0913 1] Shot effects
  (Networking|SwitchHasAuthority
    (:Remote
      ;;[0.1178 1 0] Play animations
      (Components|Animation|PlayAnimation (Variables|Default|GetSK_Weapon) _shotanimation_weapon false)
      (bind _asbp_player_character (Utilities|Casting|CastToBP_PlayerCharacter (Game|GetInstigator)))
      (Animation|Montage|PlayMontage (Default|GetVisibleMesh _asbp_player_character) (select (Pawn|IsLocallyControlled _asbp_player_character) "/Game/Client/Assets/Character/FirstPersonArms/Animations/FP_Rifle_Shoot_Montage.FP_Rifle_Shoot_Montage" _shotanimation_character)))))

(event Custom|StopShooting_Server
  ;[0 1 0.05611] Shooting
  (Utilities|Time|ClearandInvalidateTimerbyHandle (Variables|Internal|GetShootingTimer)))

(event Custom|Init_server
  ;[0 1 0.1939] Initial
)

(event Custom|TraceDEBUG_Multicast
  (params (Center :type Vector) (LineStart :type Vector) (LineEnd :type Vector))
  ;[1 0 0] Debug
  (Rendering|Debug|DrawDebugSphere Center 5.0 12 "(R=1.000000,G=0.000000,B=0.000000,A=1.000000)" 5.0))

(event Custom|StartShot_Server
  (bind _weapondefinition (Variables|Default|GetWeaponDefinition))
  (bind (_shotrate _auto) (Utilities|Struct|Breakstr_WeaponDefinition _weapondefinition))
  ;[0 1 0.05611] Shooting
  (if (and (not (Variables|Internal|GetCooldown)) (not (Variables|Internal|GetReload)))
    ;;[0.7882 0 1] Cooldown
    (Variables|Internal|SetCooldown true)
    (Utilities|Time|SetTimerbyFunctionName 0 "ResetCooldown" (.ShotRate (Utilities|Struct|Breakstr_WeaponDefinition (Variables|Default|GetWeaponDefinition))))
    (Internal|Shot)
    (if _auto
      (bind _returnvalue (Utilities|Time|SetTimerbyFunctionName 0 "Shot" _shotrate true))
      (Variables|Internal|SetShootingTimer _returnvalue))))

(event Custom|PlayReloadEffects
  (bind _weapondefinition (Variables|Default|GetWeaponDefinition))
  (bind (_reloadanimation_weapon _reloadanimation_character) (Utilities|Struct|Breakstr_WeaponDefinition _weapondefinition))
  ;[0 1 0.1429] Reload effects
  ;;[1 0.3065 0.9684] Play animations
  (Components|Animation|PlayAnimation (Variables|Default|GetSK_Weapon) _reloadanimation_weapon false)
  (bind _asbp_player_character (Utilities|Casting|CastToBP_PlayerCharacter (Game|GetInstigator)))
  (Animation|Montage|PlayMontage (Default|GetVisibleMesh _asbp_player_character) (select (Pawn|IsLocallyControlled _asbp_player_character) "/Game/Client/Assets/Animations/UE5_Reload_Rifle_Montage.UE5_Reload_Rifle_Montage" _reloadanimation_character)))

(event Custom|Reload_Server
  ;[1 0.8684 0.1637] Reload
  ;;[0 0.09559 1] Check reload
  (if (Math|Boolean|ANDBoolean (not (Variables|Internal|GetCooldown)) (not (Variables|Internal|GetReload)) (> (Variables|Weapon|Ammo|GetTotalAmmo) 0))
    (Variables|Internal|SetReload true)
    (Utilities|Time|SetTimerbyFunctionName 0 "ResetReloadTimer" (.ReloadTime (Utilities|Struct|Breakstr_WeaponDefinition (Variables|Default|GetWeaponDefinition))))
    (Internal|ReloadCountingAmmo)
    (CallFunction|ReloadMulticast)))

(event Custom|Reload_Multicast
  ;[1 0.8684 0.1637] Reload
  (Networking|SwitchHasAuthority
    (:Remote
      (CallFunction|PlayReloadEffects))))

(event EventBeginPlay
  (bind _weapondefinition (Variables|Default|GetWeaponDefinition))
  (bind (_shotrange _ammo _maxammo) (Utilities|Struct|Breakstr_WeaponDefinition _weapondefinition))
  ;[0 1 0.1939] Initial
  (Internal|Init)
  (Networking|SwitchHasAuthority
    (:Authority
      (Variables|Weapon|Ammo|SetCurrentAmmo _ammo)
      (Variables|Weapon|Ammo|SetTotalAmmo _maxammo)
      (Utilities|FlowControl|DelayUntilNextTick)
      (Default|CallOnChangeAmmo (Variables|Weapon|Ammo|GetCurrentAmmo) (Variables|Weapon|Ammo|GetTotalAmmo)))))

(fn ConstructionScript)

(fn Init
  (if (not (Networking|IsServer))
    (Components|SkeletalMesh|SetSkeletalMeshAsset (Variables|Default|GetSK_Weapon) (.Mesh (Utilities|Struct|Breakstr_WeaponDefinition (Variables|Default|GetWeaponDefinition))))
    (CallFunction|InitServer)))

(fn ResetCooldown
  (Variables|Internal|SetCooldown false))

(fn Shot
  (if (Internal|ConditionsOfShot)
    (Internal|CountingAmmo)
    (bind _outhit (Internal|GetTrice))
    (bind _output_get (LocalVariables|SetHitResult _outhit))
    ;[1 0 0] Debug ONLY
    (CallFunction|TraceDEBUGMulticast (.Location (Collision|BreakHitResult _output_get)) (.TraceStart (Collision|BreakHitResult _output_get)) (.TraceEnd (Collision|BreakHitResult _output_get)))
    ;[0.1851 0.2187 1] Show visual effects
    (CallFunction|ShotMulticast)
    (Default|CallOnHit (LocalVariables|GetHitResult) (.Damage (Utilities|Struct|Breakstr_WeaponDefinition (Variables|Default|GetWeaponDefinition))))
    (else
      (CallFunction|StopShootingServer)
      (CallFunction|ReloadServer)
      (return))))

(fn ConditionsOfShot
  (return (> (Variables|Weapon|Ammo|GetCurrentAmmo) 0)))

(fn CountingAmmo
  (Math|Integer|DecrementInt (Variables|Weapon|Ammo|GetCurrentAmmo)
    (:%20%20
      (Default|CallOnChangeAmmo (Variables|Weapon|Ammo|GetCurrentAmmo) (Variables|Weapon|Ammo|GetTotalAmmo)))))

(fn ReloadCountingAmmo
  (bind _weapondefinition (Variables|Default|GetWeaponDefinition))
  (bind _ammo (Utilities|Struct|Breakstr_WeaponDefinition _weapondefinition))
  (LocalVariables|SetPreviosAmmo (Variables|Weapon|Ammo|GetCurrentAmmo))
  (Variables|Weapon|Ammo|SetCurrentAmmo (Math|Integer|Min(Integer) (Variables|Weapon|Ammo|GetTotalAmmo) _ammo))
  (Variables|Weapon|Ammo|SetTotalAmmo (Math|Integer|Max(Integer) (- (+ (Variables|Weapon|Ammo|GetTotalAmmo) (LocalVariables|GetPreviosAmmo)) _ammo)))
  (Default|CallOnChangeAmmo (Variables|Weapon|Ammo|GetCurrentAmmo) (Variables|Weapon|Ammo|GetTotalAmmo)))

(fn ResetReloadTimer
  (Variables|Internal|SetReload false))

(fn GetTrice
  (bind _weapondefinition (Variables|Default|GetWeaponDefinition))
  (bind _shotrange (Utilities|Struct|Breakstr_WeaponDefinition _weapondefinition))
  (bind _asbp_player_character (Utilities|Casting|CastToBP_PlayerCharacter (Game|GetInstigator))
    (:then
      (bind _outhit (Collision|LineTraceForObjects (Transformation|GetWorldLocation (Variables|/Game/Client/Blueprints/Game/BP_PlayerCharacter.BP_PlayerCharacter_C|GetCamera _asbp_player_character)) (+ (Transformation|GetWorldLocation (Variables|/Game/Client/Blueprints/Game/BP_PlayerCharacter.BP_PlayerCharacter_C|GetCamera _asbp_player_character)) (* (Transformation|GetActorForwardVector (Pawn|GetController _asbp_player_character)) (Math|Vector|MakeVector _shotrange _shotrange _shotrange))) (Utilities|Array|MakeArray "ObjectTypeQuery1" "ObjectTypeQuery2" "ObjectTypeQuery3") true (Utilities|Array|MakeArray (Game|GetInstigator)) "None"))
      (return _outhit))
    (:CastFailed
      (return ""))))